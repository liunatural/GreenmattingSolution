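; BP_HXGreenMatting is an actor that shows a live video texture on a plane, apparently for green-screen matting.
; On BeginPlay it connects to a hardcoded localhost stream, prints the result and creates a dynamic Mat_LiveStream instance on the plane.
; Each Tick it pushes GetLiveTexture's result into that material's texture parameter, spelled "LiveSteam".
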(event `self.ReceiveBeginPlay`
  (bind _returnvalue (`self.Connect` "127.0.0.1" "10002"))
  (`KismetSystemLibrary.PrintString` (`KismetStringLibrary.Conv_BoolToString` _returnvalue) true false)
  (bind _returnvalue_2 (`PrimitiveComponent.CreateDynamicMaterialInstance` (`self.Plane`) 0 "/Game/GreenMatting/Mat_LiveStream.Mat_LiveStream"))
  (set `self.Dynamic_Material` _returnvalue_2))

(event `self.ReceiveTick`
  (params (DeltaSeconds :type "Float (single-precision)"))
  (`/Engine/EditorBlueprintResources/StandardMacros.IsValid` (`self.Dynamic_Material`)
    (:`Is Valid`
      (bind _returnvalue (`self.GetLiveTexture`))
      (`MaterialInstanceDynamic.SetTextureParameterValue` (`self.Dynamic_Material`) "LiveSteam" _returnvalue))))

(fn `UserConstructionScript`)